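; BP_trace is an experimental Blueprint for line tracing and event-driven spawning or movement.
; Left mouse fires a debug-drawn Visibility trace forward from AddArrow, but its result is unused.
; Ev_Click switches on Selection to either add mesh and particle components or flip-flop the Position timeline, sliding StaticMesh along X.
; Evt_Test is a similar switch fixed to the component-adding branch, and nothing here calls either event.
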(event `Key|LeftMouseButton`
  (params (Key :type "Key Structure"))
  (bind _add_arrow (`self.Add_Arrow`))
  (bind _returnvalue (`SceneComponent.K2_GetComponentLocation` _add_arrow))
  ;[0.2384 0.05286 0.05127 1 15] Trigger_command_
  (:`Pressed`
    (bind _outhit (`KismetSystemLibrary.LineTraceSingle` :`Start` _returnvalue :`End` (+ _returnvalue (* (`SceneComponent.GetForwardVector` _add_arrow) 500.0)) :`TraceChannel` "TraceTypeQuery1" :`DrawDebugType` "ForDuration"))))

(event `Ev_Click`
  (switch `int` (`self.Selection`)
    (:`0`
      (`AddComponent|NODE_AddStaticMeshComponent-0` :`self` (`self.Static_Mesh`))
      (`AddComponent|NODE_AddParticleSystemComponent-0`))
    (:`1`
      (`/Engine/EditorBlueprintResources/StandardMacros.FlipFlop`
        (:`A`
          (bind (_direction _newtrack_0) (`Timeline|Position` :!label _label)
            (:`Update`
              (`self.K2_SetActorRelativeLocation` (`self.Static_Mesh`) (`KismetMathLibrary.MakeVector` (* _newtrack_0 50.0)) false false))))
        (:`B`
          (goto _label :!via `Reverse`))))))

(event `Evt_Test`
  ;[0.2122 0.03311 0.0319 1 10] Custom_Event_Add
  ;[0.2307 0.2346 0.03955 1 10] Event_Switch
  (switch `int` 0
    (:`0`
      ;[0.0999 0.2502 0.3968 1 10] Add_Static_Mesh
      (`AddComponent|NODE_AddStaticMeshComponent-1`)
      ;[0.05286 0.1046 0.147 1 10] Add_Particle
      (`AddComponent|NODE_AddParticleSystemComponent-1`))
    (:`1`
      ;[0.4852 0.3613 0.1195 1 10] Time_Add_and_Setting
      (`Timeline|Timeline`))))

(fn `UserConstructionScript`)