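; BP_Enermy_Attack is an enemy pawn that continuously follows the player.
; On BeginPlay it runs AI MoveTo toward the first player's pawn, retrying 0.2 seconds after either success or failure.
; An unconnected debug line trace from AttackArrow on the Visibility channel never runs and its hit result is unused, so no attack logic is active.
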(event `self.ReceiveTick`
  (params (DeltaSeconds :type "Float (single-precision)")))

(event `self.ReceiveBeginPlay`
  ;[0.8281 0.6562 1] Player_Follow_AI_
  (`|AIMoveTo` self (0.0 0.0 0.0) (`GameplayStatics.GetPlayerPawn` 0) :!label _label
    (:`OnSuccess`
      _)
    (:`OnFail`
      _))
  (`KismetSystemLibrary.Delay` 0.2)
  (goto _label))

(fn `UserConstructionScript`)