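; BP_Door is a sliding door that splits into four mesh panels when an actor overlaps its Box trigger.
; The Door_Open_ timeline drives Lerps on relative location, moving the top and bottom center panels apart vertically and the left and right panels apart along X.
; End overlap calls Play on the same timeline instead of Reverse, so the graph has no closing motion.
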(event `self.Box.OnComponentBeginOverlap`
  (params (OverlappedComponent :type "PrimitiveComponent Object Reference") (OtherActor :type "Actor Object Reference") (OtherComp :type "PrimitiveComponent Object Reference") (OtherBodyIndex :type Integer) (bFromSweep :type Boolean) (SweepResult :type "HitResult Structure (by ref)"))
  (bind (_direction _newtrack_0) (`Timeline|Door_Open_` :!label _label)
    (:`Update`
      (`SceneComponent.K2_SetRelativeLocation` (`self.SM_Door_Center_Top`) (`KismetMathLibrary.MakeVector` 0.0 0.0 (`KismetMathLibrary.Lerp` 0.0 140.0 _newtrack_0)) false false)
      (`SceneComponent.K2_SetRelativeLocation` (`self.SM_Door_Center_Bottom`) (`KismetMathLibrary.MakeVector` 0.0 0.0 (`KismetMathLibrary.Lerp` 0.0 -200.0 _newtrack_0)) false false)
      (`SceneComponent.K2_SetRelativeLocation` (`self.SM_Door_Right`) (`KismetMathLibrary.MakeVector` (`KismetMathLibrary.Lerp` 0.0 50.0 _newtrack_0)) false false)
      (`SceneComponent.K2_SetRelativeLocation` (`self.SM_Door_Left`) (`KismetMathLibrary.MakeVector` (`KismetMathLibrary.Lerp` 0.0 -50.0 _newtrack_0)) false false))))

(event `self.Box.OnComponentEndOverlap`
  (params (OverlappedComponent :type "PrimitiveComponent Object Reference") (OtherActor :type "Actor Object Reference") (OtherComp :type "PrimitiveComponent Object Reference") (OtherBodyIndex :type Integer))
  (goto _label))

(fn `UserConstructionScript`)